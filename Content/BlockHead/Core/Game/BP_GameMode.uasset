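; BlockHead game mode that runs the HUD, level progression, pause menu and win/lose screens.
; BeginPlay creates the HUD, caches player and game instance, and sets game input.
; LevelComplete shows a widget, then a timed LoadNextLevel asks the game instance for the next level or ends with a win.
; It also restarts from the first level, toggles pause, and derives score from the player's X position.
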(event `self.ReceiveBeginPlay`
  ;[0.1399 0.9115 0.2176 0.7565] Begin Play Sequence
  (`|ExecutionSequence`
    (:`then_0`
      ;[0.1399 0.9115 0.2176 0.7565] Add HUD to Viewport
      (bind _returnvalue (`|CreateWidget` "/Game/BlockHead/Core/UI/WBP_HUD.WBP_HUD_C"))
      (set `self.HUD` _returnvalue)
      (`UserWidget.AddToViewport` (`self.HUD`) 0))
    (:`then_1`
      ;[0.1399 0.9115 0.2176 0.7565] Get Reference to Player Pawn
      (bind _asbp_player (cast `/Game/BlockHead/Core/Actors/BP_Player` (`GameplayStatics.GetPlayerPawn` 0)))
      (set `self.Player` _asbp_player))
    (:`then_2`
      ;[0.1399 0.9115 0.2176 0.7565] Get Reference to Game Instance
      (bind _asbp_game_instance (cast `/Game/BlockHead/Core/Game/BP_GameInstance` (`GameplayStatics.GetGameInstance`)))
      (set `self.GameInstance` _asbp_game_instance))
    (:`then_3`
      ;[0.1399 0.9115 0.2176 0.7565] Input Mode = Game
      (`/Game/BlockHead/Core/Game/BP_GameInstance.InputModeGame` (`self.GameInstance`)))))

(fn `GameComplete`
  (params (bPlayerWon :type Boolean))
  ;[0.1399 0.9115 0.2176 0.7565] Game is Complete - Show End Menu: Did Player Win or Lose?
  (if bPlayerWon
    (bind _returnvalue (`|CreateWidget` "/Game/BlockHead/Core/UI/WBP_GameComplete.WBP_GameComplete_C" null "You Won! :)"))
    (`UserWidget.AddToViewport` _returnvalue 0)
    (else
      (bind _returnvalue_2 (`|CreateWidget` "/Game/BlockHead/Core/UI/WBP_GameComplete.WBP_GameComplete_C" null "You Lost! :("))
      (`UserWidget.AddToViewport` _returnvalue_2 0)))
  (`/Game/BlockHead/Core/Game/BP_GameInstance.InputModeUI` (`self.GameInstance`))
  (return))

(fn `GetScoreAsText`
  (returns (CurrentScore :type Text))
  (bind _returnvalue_x (`KismetMathLibrary.BreakVector` (`self.K2_GetActorLocation` (`self.Player`))))
  (return (`|GenericToText` (`KismetMathLibrary.Round64` (/ _returnvalue_x 500.0)))))

(fn `LevelComplete`
  ;[0.1399 0.9115 0.2176 0.7565] Show Level Complete Widget and Set Timer for Loading Next Level
  (bind _returnvalue (`|CreateWidget` "/Game/BlockHead/Core/UI/WBP_LevelComplete.WBP_LevelComplete_C"))
  (`UserWidget.AddToViewport` _returnvalue 0)
  (`KismetSystemLibrary.K2_SetTimer` null "LoadNextLevel" 2.0)
  (return))

(fn `LoadNextLevel`
  (bind _bfinallevel (`/Game/BlockHead/Core/Game/BP_GameInstance.IsPlayerOnFinalLevel` (`self.GameInstance`)))
  (if _bfinallevel
    (`self.GameComplete` true)
    (else
      (`/Game/BlockHead/Core/Game/BP_GameInstance.NextLevel` (`self.GameInstance`))
      (bind _levelname (`/Game/BlockHead/Core/Game/BP_GameInstance.GetLevelName` (`self.GameInstance`)))
      (`GameplayStatics.OpenLevel` _levelname)))
  (return))

(fn `PauseGame`
  (bind _pausemenu (`self.PauseMenu`))
  (if (`self.GamePaused`)
    (`/Engine/EditorBlueprintResources/StandardMacros.IsValid` _pausemenu
      (:`Is Valid`
        (`Widget.RemoveFromParent` _pausemenu)
        (bind _output_get (set `self.GamePaused` false))
        (`GameplayStatics.SetGamePaused` _output_get)
        (`/Game/BlockHead/Core/Game/BP_GameInstance.InputModeGame` (`self.GameInstance`))))
    (else
      (bind _returnvalue (`|CreateWidget` "/Game/BlockHead/Core/UI/WBP_GamePaused.WBP_GamePaused_C"))
      (bind _output_get_2 (set `self.PauseMenu` _returnvalue))
      (`UserWidget.AddToViewport` _output_get_2 0)
      (`/Game/BlockHead/Core/Game/BP_GameInstance.InputModePaused` (`self.GameInstance`))
      (bind _output_get_3 (set `self.GamePaused` true))
      (`GameplayStatics.SetGamePaused` _output_get_3)))
  (return))

(fn `RestartGame`
  ;[0.1399 0.9115 0.2176 0.7565] Restart: Input Mode Set to Game. Reset Level Number and Load the First Level
  (`/Game/BlockHead/Core/Game/BP_GameInstance.InputModeGame` (`self.GameInstance`))
  (`/Game/BlockHead/Core/Game/BP_GameInstance.ResetInstance` (`self.GameInstance`))
  (bind _levelname (`/Game/BlockHead/Core/Game/BP_GameInstance.GetLevelName` (`self.GameInstance`)))
  (`GameplayStatics.OpenLevel` _levelname))

(fn `UserConstructionScript`)